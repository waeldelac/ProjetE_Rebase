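; BP_Nuke is an actor that displays a nuke effect with an animation triggered by the W key.
; The construction script gives the Nuke0 component a dynamic M_Nuke material, which BeginPlay sets up with fixed shape, distortion and blue glow parameters.
; It enables player input, and W plays a timeline that drives the root's world location from its Scale track and Z scale from PosZ, with X and Y scale at zero.
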(event `self.ReceiveBeginPlay`
  (bind _mat_inst (`self.Mat_Inst`))
  (`MaterialInstanceDynamic.SetScalarParameterValue` _mat_inst "distort" 20.0)
  (`MaterialInstanceDynamic.SetScalarParameterValue` _mat_inst "divide" 100.0)
  (`MaterialInstanceDynamic.SetScalarParameterValue` _mat_inst "max" 80.0)
  (`MaterialInstanceDynamic.SetScalarParameterValue` _mat_inst "min" 0.6)
  (`MaterialInstanceDynamic.SetScalarParameterValue` _mat_inst "multiply" 215.0)
  (`MaterialInstanceDynamic.SetScalarParameterValue` _mat_inst "power" 3.0)
  (`MaterialInstanceDynamic.SetScalarParameterValue` _mat_inst "width" 0.0)
  (`MaterialInstanceDynamic.SetScalarParameterValue` _mat_inst "x" 0.0)
  (`MaterialInstanceDynamic.SetScalarParameterValue` _mat_inst "y" 0.0)
  (`MaterialInstanceDynamic.SetScalarParameterValue` _mat_inst "z" 100.0)
  (`MaterialInstanceDynamic.SetVectorParameterValue` _mat_inst "Base_Color" (struct :`G` 5.75 :`B` 20.0 :`A` 1.0))
  (`self.EnableInput` (`GameplayStatics.GetPlayerController` 0)))

(event `Key|W`
  (params (Key :type "Key Structure"))
  (:`Pressed`
    (bind (_direction _scale _pos_z) (`Timeline|Timeline_0`)
      (:`Update`
        (`SceneComponent.K2_SetWorldLocation` (`self.DefaultSceneRoot`) (`KismetMathLibrary.Conv_DoubleToVector` _scale) false false)
        (`SceneComponent.SetWorldScale3D` (`self.DefaultSceneRoot`) (`KismetMathLibrary.MakeVector` 0.0 0.0 _pos_z))))))

(fn `UserConstructionScript`
  (bind _returnvalue (`PrimitiveComponent.CreateDynamicMaterialInstance` (`self.nuke_0`) 0 "/Game/Blob/Nico/Nuke/M_Nuke.M_Nuke" "None"))
  (set `self.Mat_Inst` _returnvalue))