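; BP_Nuke_Scale is a nuke effect actor that animates a top and bottom mesh, triggered by pressing L.
; Construction gives both meshes dynamic M_TranslucentNuke instances and enables custom depth; BeginPlay makes them transparent, with opposite Speed values.
; The Scale timeline grows both meshes, offsets the top along Z and drives opacity, then sets the top's final relative location.
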(event `self.ReceiveBeginPlay`
  (`MaterialInstanceDynamic.SetScalarParameterValue` (`self.Haut`) "ColorPower" 5000.0)
  (`MaterialInstanceDynamic.SetScalarParameterValue` (`self.Bas`) "ColorPower" 5000.0)
  (`MaterialInstanceDynamic.SetScalarParameterValue` (`self.Haut`) "DepthBias" -1.0)
  (`MaterialInstanceDynamic.SetScalarParameterValue` (`self.Bas`) "DepthBias" -1.0)
  (`MaterialInstanceDynamic.SetScalarParameterValue` (`self.Haut`) "Opacity" 0.0)
  (`MaterialInstanceDynamic.SetScalarParameterValue` (`self.Bas`) "Opacity" 0.0)
  (`MaterialInstanceDynamic.SetScalarParameterValue` (`self.Haut`) "width" 3.0)
  (`MaterialInstanceDynamic.SetScalarParameterValue` (`self.Bas`) "width" 3.0)
  (`MaterialInstanceDynamic.SetScalarParameterValue` (`self.Haut`) "Speed" 200.0)
  (`MaterialInstanceDynamic.SetScalarParameterValue` (`self.Bas`) "Speed" -200.0)
  (`self.EnableInput` (`GameplayStatics.GetPlayerController` 0)))

(event `Key|L`
  (params (Key :type "Key Structure"))
  (:`Pressed`
    (`MaterialInstanceDynamic.SetScalarParameterValue` (`self.Haut`) "Opacity" 0.7)
    (`MaterialInstanceDynamic.SetScalarParameterValue` (`self.Bas`) "Opacity" 0.7)
    (`KismetSystemLibrary.PrintString` "Hello")
    (bind (_direction _scalebas _scalehaut _positionz _opacity) (`Timeline|scale` :!via `PlayFromStart`)
      (:`Update`
        (bind _returnvalue (/ _scalebas 2.0))
        (`SceneComponent.SetRelativeScale3D` (`self.bas_de_nuke`) (`KismetMathLibrary.MakeVector` _returnvalue _returnvalue _scalebas))
        (`SceneComponent.SetRelativeScale3D` (`self.haut_de_nuke`) (`KismetMathLibrary.Conv_DoubleToVector` _scalehaut))
        (`SceneComponent.K2_AddLocalOffset` (`self.haut_de_nuke`) (`KismetMathLibrary.MakeVector` 0.0 0.0 _positionz) false false)
        (`MaterialInstanceDynamic.SetScalarParameterValue` (`self.Haut`) "Opacity" _opacity)
        (`MaterialInstanceDynamic.SetScalarParameterValue` (`self.Bas`) "Opacity" _opacity))
      (:`Finished`
        (`SceneComponent.K2_SetRelativeLocation` (`self.haut_de_nuke`) (0.0 0.0 970.0) false false)))))

(fn `UserConstructionScript`
  (bind _returnvalue (`PrimitiveComponent.CreateDynamicMaterialInstance` (`self.haut_de_nuke`) 0 "/Game/Blob/Nico/Nuke/M_TranslucentNuke.M_TranslucentNuke" "None"))
  (set `self.Haut` _returnvalue)
  (bind _returnvalue_2 (`PrimitiveComponent.CreateDynamicMaterialInstance` (`self.bas_de_nuke`) 0 "/Game/Blob/Nico/Nuke/M_TranslucentNuke.M_TranslucentNuke" "None"))
  (set `self.Bas` _returnvalue_2)
  (`PrimitiveComponent.SetRenderCustomDepth` (`self.bas_de_nuke`) true)
  (`PrimitiveComponent.SetRenderCustomDepth` (`self.haut_de_nuke`) true)
  (`PrimitiveComponent.SetCustomDepthStencilWriteMask` (`self.haut_de_nuke`) "ERSM_Default")
  (`PrimitiveComponent.SetCustomDepthStencilWriteMask` (`self.bas_de_nuke`) "ERSM_Default")
  (`PrimitiveComponent.SetCustomDepthStencilValue` (`self.haut_de_nuke`) 0)
  (`PrimitiveComponent.SetCustomDepthStencilValue` (`self.bas_de_nuke`) 0))