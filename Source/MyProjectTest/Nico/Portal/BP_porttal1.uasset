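; Portal actor that teleports a DefaultPawn hitting it to a BP_porttal2 with the same PortalIndex, seeking a non-entrance one.
; The construction script positions the portal and exit points C1 and C2 and caches the partner.
; Hit picks the destination's C1 or C2 by which local point is nearer, then offsets control yaw from exit rotations.
; Partner-camera rotation experiments are disconnected, and debug prints remain.
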(event `self.ReceiveTick`
  (params (DeltaSeconds :type "Float (single-precision)")))

(event `self.ReceiveBeginPlay`
  (`self.EnableInput` (`GameplayStatics.GetPlayerController` 0))
  (bind _outactors (`GameplayStatics.GetAllActorsOfClass` "/Game/Blob/Nico/Portal/BP_porttal2.BP_porttal2_C"))
  (for _array_element _outactors
    (if (== (`/Game/Blob/Nico/Portal/BP_porttal2.PortalIndex` _array_element) (`self.PortalIndex`))
      (set `self.OtherPortal` _array_element)
      (break))))

(event `self.ReceiveHit`
  (params (MyComp :type "PrimitiveComponent Object Reference") (Other :type "Actor Object Reference") (OtherComp :type "PrimitiveComponent Object Reference") (bSelfMoved :type Boolean) (HitLocation :type "Vector Structure") (HitNormal :type "Vector Structure") (NormalImpulse :type "Vector Structure") (Hit :type "HitResult Structure (by ref)"))
  (bind (_returnvalue_roll _returnvalue_pitch _returnvalue_yaw) (`KismetMathLibrary.BreakRotator` (`self.K2_GetActorRotation` (`GameplayStatics.GetPlayerController` 0))))
  (bind (_returnvalue_roll_2 _returnvalue_pitch_2 _returnvalue_yaw_2) (`KismetMathLibrary.BreakRotator` (`self.K2_GetActorRotation` (`GameplayStatics.GetPlayerController` 0))))
  (bind (_returnvalue_roll_3 _returnvalue_pitch_3 _returnvalue_yaw_3) (`KismetMathLibrary.BreakRotator` (`self.K2_GetActorRotation` (`GameplayStatics.GetPlayerController` 0))))
  (bind (_returnvalue_roll_4 _returnvalue_pitch_4 _returnvalue_yaw_4) (`KismetMathLibrary.BreakRotator` (`self.K2_GetActorRotation` (`GameplayStatics.GetPlayerController` 0))))
  (bind (_returnvalue_roll_5 _returnvalue_pitch_5 _returnvalue_yaw_5) (`KismetMathLibrary.BreakRotator` (`SceneComponent.K2_GetComponentRotation` (`self.C2`))))
  (bind (_returnvalue_roll_6 _returnvalue_pitch_6 _returnvalue_yaw_6) (`KismetMathLibrary.BreakRotator` (`SceneComponent.K2_GetComponentRotation` (`self.C1`))))
  (bind (_returnvalue_roll_7 _returnvalue_pitch_7 _returnvalue_yaw_7) (`KismetMathLibrary.BreakRotator` (`SceneComponent.K2_GetComponentRotation` (`self.C2`))))
  (bind (_returnvalue_roll_8 _returnvalue_pitch_8 _returnvalue_yaw_8) (`KismetMathLibrary.BreakRotator` (`SceneComponent.K2_GetComponentRotation` (`self.C1`))))
  (bind _returnvalue (`SceneComponent.K2_GetComponentLocation` (`DefaultPawn.MeshComponent` (`self.MyPawn`))))
  (bind _asdefault_pawn (cast `DefaultPawn` Other))
  (set `self.MyPawn` _asdefault_pawn)
  (if (< (`KismetMathLibrary.Vector_Distance` (`SceneComponent.K2_GetComponentLocation` (`self.C2`)) _returnvalue) (`KismetMathLibrary.Vector_Distance` _returnvalue (`SceneComponent.K2_GetComponentLocation` (`self.C1`))))
    (`KismetSystemLibrary.PrintString` "Hello")
    (if (`self.Entrance`)
      (bind _outactors (`GameplayStatics.GetAllActorsOfClass` "/Game/Blob/Nico/Portal/BP_porttal2.BP_porttal2_C"))
      (for _array_element _outactors
        (if (and (== (`/Game/Blob/Nico/Portal/BP_porttal2.PortalIndex` _array_element) (`self.PortalIndex`)) (not (`/Game/Blob/Nico/Portal/BP_porttal2.Entrance` _array_element)))
          (break)))
      (bind _c1 (`/Game/Blob/Nico/Portal/BP_porttal2.C1` _array_element))
      (`self.K2_SetActorLocation` (`self.MyPawn`) (`SceneComponent.K2_GetComponentLocation` _c1) false false)
      (`KismetSystemLibrary.PrintString` (`KismetStringLibrary.Conv_DoubleToString` _returnvalue_yaw_3))
      (`KismetSystemLibrary.PrintString` (`KismetStringLibrary.Conv_DoubleToString` 0.0))
      (bind (_returnvalue_roll_9 _returnvalue_pitch_9 _returnvalue_yaw_9) (`KismetMathLibrary.BreakRotator` (`SceneComponent.K2_GetComponentRotation` _c1)))
      (`KismetSystemLibrary.PrintString` (`KismetStringLibrary.Conv_DoubleToString` _returnvalue_yaw_9))
      (`Controller.SetControlRotation` (`GameplayStatics.GetPlayerController` 0) (`KismetMathLibrary.MakeRotator` 0.0 0.0 (+ _returnvalue_yaw_3 _returnvalue_yaw_6 (- _returnvalue_yaw_6 _returnvalue_yaw_9))))
      (`KismetSystemLibrary.PrintString` (`KismetStringLibrary.Conv_DoubleToString` _returnvalue_yaw_3))
      (else
        (bind _outactors_2 (`GameplayStatics.GetAllActorsOfClass` "/Game/Blob/Nico/Portal/BP_porttal2.BP_porttal2_C"))
        (for _array_element_2 _outactors_2
          (if (and (== (`/Game/Blob/Nico/Portal/BP_porttal2.PortalIndex` _array_element_2) (`self.PortalIndex`)) (and (not (`/Game/Blob/Nico/Portal/BP_porttal2.Entrance` _array_element_2)) (not (`self.Entrance`))))
            (break)))
        (bind _c1_2 (`/Game/Blob/Nico/Portal/BP_porttal2.C1` _array_element_2))
        (`self.K2_SetActorLocation` (`self.MyPawn`) (`SceneComponent.K2_GetComponentLocation` _c1_2) false false)
        (bind (_returnvalue_roll_10 _returnvalue_pitch_10 _returnvalue_yaw_10) (`KismetMathLibrary.BreakRotator` (`SceneComponent.K2_GetComponentRotation` _c1_2)))
        (`Controller.SetControlRotation` (`GameplayStatics.GetPlayerController` 0) (`KismetMathLibrary.MakeRotator` 0.0 0.0 (+ _returnvalue_yaw_2 _returnvalue_yaw_7 (- _returnvalue_yaw_7 _returnvalue_yaw_10))))))
    (else
      (`KismetSystemLibrary.PrintString` "bye")
      (if (`self.Entrance`)
        (bind _outactors_3 (`GameplayStatics.GetAllActorsOfClass` "/Game/Blob/Nico/Portal/BP_porttal2.BP_porttal2_C"))
        (for _array_element_3 _outactors_3
          (if (and (== (`/Game/Blob/Nico/Portal/BP_porttal2.PortalIndex` _array_element_3) (`self.PortalIndex`)) (not (`/Game/Blob/Nico/Portal/BP_porttal2.Entrance` _array_element_3)))
            (break)))
        (bind _c2 (`/Game/Blob/Nico/Portal/BP_porttal2.C2` _array_element_3))
        (`self.K2_SetActorLocation` (`self.MyPawn`) (`SceneComponent.K2_GetComponentLocation` _c2) false false)
        (bind (_returnvalue_roll_11 _returnvalue_pitch_11 _returnvalue_yaw_11) (`KismetMathLibrary.BreakRotator` (`SceneComponent.K2_GetComponentRotation` _c2)))
        (`Controller.SetControlRotation` (`GameplayStatics.GetPlayerController` 0) (`KismetMathLibrary.MakeRotator` 0.0 0.0 (+ _returnvalue_yaw_4 _returnvalue_yaw_8 (- _returnvalue_yaw_8 _returnvalue_yaw_11))))
        (else
          (bind _outactors_4 (`GameplayStatics.GetAllActorsOfClass` "/Game/Blob/Nico/Portal/BP_porttal2.BP_porttal2_C"))
          (for _array_element_4 _outactors_4
            (if (and (== (`/Game/Blob/Nico/Portal/BP_porttal2.PortalIndex` _array_element_4) (`self.PortalIndex`)) (and (not (`/Game/Blob/Nico/Portal/BP_porttal2.Entrance` _array_element_4)) (not (`self.Entrance`))))
              (break)))
          (bind _c2_2 (`/Game/Blob/Nico/Portal/BP_porttal2.C2` _array_element_4))
          (`self.K2_SetActorLocation` (`self.MyPawn`) (`SceneComponent.K2_GetComponentLocation` _c2_2) false false)
          (bind _returnvalue_roll_12 (`KismetMathLibrary.BreakRotator` (`SceneComponent.K2_GetComponentRotation` _c2_2)))
          (`Controller.SetControlRotation` (`GameplayStatics.GetPlayerController` 0) (`KismetMathLibrary.MakeRotator` 0.0 0.0 (+ _returnvalue_yaw _returnvalue_yaw_5 (- _returnvalue_yaw_5 _returnvalue_roll_12)))))))))

(fn `UserConstructionScript`
  ;[1 1 1] Set locations
  (`SceneComponent.K2_SetRelativeTransform` (`self.portal`) (`self.PortalTransform`) false false)
  (`SceneComponent.K2_SetRelativeLocation` (`self.C1`) (`self.Exit1`) false false)
  (`SceneComponent.K2_SetRelativeLocation` (`self.C2`) (`self.Exit2`) false false)
  (bind _outactors (`GameplayStatics.GetAllActorsOfClass` "/Game/Blob/Nico/Portal/BP_porttal2.BP_porttal2_C"))
  (for _array_element _outactors
    (if (== (`/Game/Blob/Nico/Portal/BP_porttal2.PortalIndex` _array_element) (`self.PortalIndex`))
      (set `self.OtherPortal` _array_element))))