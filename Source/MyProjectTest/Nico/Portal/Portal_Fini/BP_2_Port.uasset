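; Linked two-gate portal actor that teleports overlapping actors between its ends and turns player 0's view to the exit arrow's yaw.
; A trigger box reveals both ends, scales them up by timeline and arms teleporting.
; Gate1 re-arms after a short delay, while Gate2 leaves teleporting off, then shrinks and hides both ends.
; Tick rotates each end's cube from the player camera's rotation, offset by the opposite end.
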(event `self.gate2.OnComponentBeginOverlap`
  (params (OverlappedComponent :type "PrimitiveComponent Object Reference") (OtherActor :type "Actor Object Reference") (OtherComp :type "PrimitiveComponent Object Reference") (OtherBodyIndex :type Integer) (bFromSweep :type Boolean) (SweepResult :type "HitResult Structure (by ref)"))
  (bind (_returnvalue_roll _returnvalue_pitch _returnvalue_yaw) (`KismetMathLibrary.BreakRotator` (`SceneComponent.K2_GetComponentRotation` (`self.Arrow1`))))
  (bind (_returnvalue_roll_2 _returnvalue_pitch_2) (`KismetMathLibrary.BreakRotator` (`Controller.GetControlRotation` (`GameplayStatics.GetPlayerController` 0))))
  ;[1 1 1] Téléportation
  (`KismetSystemLibrary.PrintString` "2")
  (if (`self.CanTP`)
    (set `self.CanTP` false)
    (`Controller.SetControlRotation` (`GameplayStatics.GetPlayerController` 0) (`KismetMathLibrary.MakeRotator` _returnvalue_roll_2 _returnvalue_pitch_2 _returnvalue_yaw))
    (`self.K2_SetActorLocation` OtherActor (`SceneComponent.K2_GetComponentLocation` (`self.Partie1`)) false false)
    (`KismetSystemLibrary.Delay` 2.0)
    (set `self.CanTP` false)
    (bind (_direction _scale) (`Timeline|Timeline_0` :!via `Reverse`)
      (:`Update`
        (`SceneComponent.SetWorldScale3D` (`self.Partie1`) (`KismetMathLibrary.Conv_DoubleToVector` _scale))
        (`SceneComponent.SetWorldScale3D` (`self.Partie2`) (`KismetMathLibrary.Conv_DoubleToVector` _scale)))
      (:`Finished`
        (`SceneComponent.SetVisibility` (`self.Partie1`) false false)
        (`SceneComponent.SetVisibility` (`self.Partie2`) false false)))))

(event `self.gate1.OnComponentBeginOverlap`
  (params (OverlappedComponent :type "PrimitiveComponent Object Reference") (OtherActor :type "Actor Object Reference") (OtherComp :type "PrimitiveComponent Object Reference") (OtherBodyIndex :type Integer) (bFromSweep :type Boolean) (SweepResult :type "HitResult Structure (by ref)"))
  (bind (_returnvalue_roll _returnvalue_pitch _returnvalue_yaw) (`KismetMathLibrary.BreakRotator` (`SceneComponent.K2_GetComponentRotation` (`self.Arrow2`))))
  (bind (_returnvalue_roll_2 _returnvalue_pitch_2) (`KismetMathLibrary.BreakRotator` (`Controller.GetControlRotation` (`GameplayStatics.GetPlayerController` 0))))
  ;[1 1 1] Téléportation
  (`KismetSystemLibrary.PrintString` "1")
  (if (`self.CanTP`)
    (set `self.CanTP` false)
    (`Controller.SetControlRotation` (`GameplayStatics.GetPlayerController` 0) (`KismetMathLibrary.MakeRotator` _returnvalue_roll_2 _returnvalue_pitch_2 _returnvalue_yaw))
    (`self.K2_SetActorLocation` OtherActor (`SceneComponent.K2_GetComponentLocation` (`self.Partie2`)) false false)
    (`KismetSystemLibrary.Delay` 0.5)
    (set `self.CanTP` true)))

(event `self.ReceiveTick`
  (params (DeltaSeconds :type "Float (single-precision)"))
  (bind (_returnvalue_roll _returnvalue_pitch _returnvalue_yaw) (`KismetMathLibrary.BreakRotator` (`SceneComponent.K2_GetComponentRotation` (`self.Partie1`))))
  (bind (_returnvalue_roll_2 _returnvalue_pitch_2 _returnvalue_yaw_2) (`KismetMathLibrary.BreakRotator` (`SceneComponent.K2_GetComponentRotation` (`self.Partie2`))))
  (bind (_returnvalue_roll_3 _returnvalue_pitch_3 _returnvalue_yaw_3) (`KismetMathLibrary.BreakRotator` (`SceneComponent.K2_GetComponentRotation` (`PlayerCameraManager.TransformComponent` (`PlayerController.PlayerCameraManager` (`GameplayStatics.GetPlayerController` 0))))))
  (bind (_returnvalue_roll_4 _returnvalue_pitch_4 _returnvalue_yaw_4) (`KismetMathLibrary.BreakRotator` (`SceneComponent.K2_GetComponentRotation` (`PlayerCameraManager.TransformComponent` (`PlayerController.PlayerCameraManager` (`GameplayStatics.GetPlayerController` 0))))))
  ;[1 1 1] Orientation caméra
  (bind _alignmenttransform (`ARBlueprintLibrary.CalculateAlignmentTransform` (`SceneComponent.K2_GetComponentToWorld` (`Actor.RootComponent` (`GameplayStatics.GetPlayerController` 0))) (`SceneComponent.K2_GetComponentToWorld` (`self.Partie2`))))
  (bind (_returnvalue_x _returnvalue_y _returnvalue_z) (`KismetMathLibrary.BreakVector` (`KismetMathLibrary.Normal` (.location _alignmenttransform))))
  (`SceneComponent.K2_SetRelativeRotation` (`self.Cube2`) (`KismetMathLibrary.MakeRotator` (- (+ _returnvalue_x _returnvalue_roll_4) _returnvalue_roll) (- (+ _returnvalue_y _returnvalue_pitch_4) _returnvalue_pitch) (- (+ _returnvalue_z _returnvalue_yaw_4) _returnvalue_yaw)) false false)
  (bind _alignmenttransform_2 (`ARBlueprintLibrary.CalculateAlignmentTransform` (`SceneComponent.K2_GetComponentToWorld` (`Actor.RootComponent` (`GameplayStatics.GetPlayerController` 0))) (`SceneComponent.K2_GetComponentToWorld` (`self.Partie1`))))
  (bind (_returnvalue_x_2 _returnvalue_y_2 _returnvalue_z_2) (`KismetMathLibrary.BreakVector` (`KismetMathLibrary.Normal` (.location _alignmenttransform_2))))
  (`SceneComponent.K2_SetRelativeRotation` (`self.Cube1`) (`KismetMathLibrary.MakeRotator` (- (+ _returnvalue_x_2 _returnvalue_roll_3) _returnvalue_roll_2) (- (+ _returnvalue_y_2 _returnvalue_pitch_3) _returnvalue_pitch_2) (- (+ _returnvalue_z_2 _returnvalue_yaw_3) _returnvalue_yaw_2)) false false))

(event `self.Box.OnComponentBeginOverlap`
  (params (OverlappedComponent :type "PrimitiveComponent Object Reference") (OtherActor :type "Actor Object Reference") (OtherComp :type "PrimitiveComponent Object Reference") (OtherBodyIndex :type Integer) (bFromSweep :type Boolean) (SweepResult :type "HitResult Structure (by ref)"))
  (`KismetSystemLibrary.PrintString` "Hello")
  (`SceneComponent.SetVisibility` (`self.Partie1`) true false)
  (`SceneComponent.SetVisibility` (`self.Partie2`) true false)
  (`SceneComponent.SetVisibility` (`self.Particles2`) true false)
  (`SceneComponent.SetVisibility` (`self.Particles1`) true false)
  (set `self.CanTP` true)
  (`ActorComponent.SetAutoActivate` (`self.Particles2`) false)
  (bind (_direction _scale) (`Timeline|Scale`)
    (:`Update`
      (`SceneComponent.SetWorldScale3D` (`self.Partie1`) (`KismetMathLibrary.Conv_DoubleToVector` _scale))
      (`SceneComponent.SetWorldScale3D` (`self.Partie2`) (`KismetMathLibrary.Conv_DoubleToVector` _scale)))))

(event `self.ReceiveBeginPlay`
  (`self.EnableInput` (`GameplayStatics.GetPlayerController` 0))
  (`SceneComponent.SetVisibility` (`self.Partie1`) false false)
  (`SceneComponent.SetVisibility` (`self.Partie2`) false false)
  (`SceneComponent.SetVisibility` (`self.Particles1`) false false)
  (`SceneComponent.SetVisibility` (`self.Particles2`) false false))

(fn `UserConstructionScript`
  (`SceneComponent.SetWorldScale3D` (`self.Partie1`) (0.0 0.0 0.0))
  (`SceneComponent.SetWorldScale3D` (`self.Partie2`) (0.0 0.0 0.0))
  (set `self.CanTP` false)
  (`SceneComponent.SetVisibility` (`self.Particles1`) false false)
  (`SceneComponent.SetVisibility` (`self.Particles2`) false false))