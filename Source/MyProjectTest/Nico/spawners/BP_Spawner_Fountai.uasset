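; BP_Spawner_Fountai is a fountain spawner that, once H is pressed, keeps producing BP_Goutte drops one after another.
; Each drop spawns above BPMortar with gravity off, the M_Dissolve material and a tag from the Tag variable.
; A timeline drives the drop's scale, then gravity is enabled and, after a short delay, the cycle loops back to spawn the next drop.
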(event `self.ReceiveBeginPlay`
  (`self.EnableInput` (`GameplayStatics.GetPlayerController` 0)))

(event `Key|H`
  (params (Key :type "Key Structure"))
  (bind (_returnvalue_x _returnvalue_y _returnvalue_z) (`KismetMathLibrary.BreakVector` (`SceneComponent.K2_GetComponentLocation` (`self.BP_Mortar`))))
  (bind _drops (`/Game/Blob/Nico/gravity/BP_Goutte.Drops` (`self.CurrentDrop`)))
  (:`Pressed`
    (`KismetSystemLibrary.PrintString` "le material est au pif")
    (bind _returnvalue (`|SpawnActorFromClass` "/Game/Blob/Nico/gravity/BP_Goutte.BP_Goutte_C" (`KismetMathLibrary.MakeTransform` (`KismetMathLibrary.MakeVector` _returnvalue_x _returnvalue_y (+ _returnvalue_z 100.0))) "Undefined" "OverrideRootScale" null null :!label _label))
    (set `self.CurrentDrop` _returnvalue)
    (`PrimitiveComponent.SetEnableGravity` _drops false)
    (`PrimitiveComponent.SetMaterial` _drops 0 "/Game/Blob/Nico/disapear/M_Dissolve.M_Dissolve")
    (bind _output_get (set `Actor.Tags` (`|MakeArray` (`KismetStringLibrary.Conv_StringToName` (`self.Tag`))) (`self.CurrentDrop`)))
    (`KismetSystemLibrary.PrintString` (`KismetStringLibrary.Conv_NameToString` (`|GetArrayItem` _output_get)))
    (bind (_direction _newtrack_0) (`Timeline|Timeline_0` :!via `PlayFromStart`)
      (:`Update`
        (`SceneComponent.SetRelativeScale3D` (`/Game/Blob/Nico/gravity/BP_Goutte.Drops` (`self.CurrentDrop`)) (`KismetMathLibrary.Conv_DoubleToVector` _newtrack_0)))
      (:`Finished`
        (`PrimitiveComponent.SetEnableGravity` (`/Game/Blob/Nico/gravity/BP_Goutte.Drops` (`self.CurrentDrop`)) true)
        (`KismetSystemLibrary.Delay` 1.0)
        (goto _label)))))

(fn `UserConstructionScript`)