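; BP_Spawn_Unique is a test-style spawner that releases a single BP_Goutte drop each time J is pressed.
; It enables player input on BeginPlay, then spawns the drop near its Box with gravity and physics off and a dissolve material applied.
; The RotLoc timeline moves and pitches Plane1, then physics releases the drop.
; After a short delay, a second timeline plays in reverse to animate Plane1 again.
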(event `self.ReceiveBeginPlay`
  (`self.EnableInput` (`GameplayStatics.GetPlayerController` 0)))

(event `Key|J`
  (params (Key :type "Key Structure"))
  (bind (_returnvalue_x _returnvalue_y _returnvalue_z) (`KismetMathLibrary.BreakVector` (`SceneComponent.K2_GetComponentLocation` (`self.Box`))))
  (bind _drops (`/Game/Blob/Nico/gravity/BP_Goutte.Drops` (`self.Current Drop`)))
  (bind _drops_2 (`/Game/Blob/Nico/gravity/BP_Goutte.Drops` (`self.Current Drop`)))
  (:`Pressed`
    (bind _returnvalue (`|SpawnActorFromClass` "/Game/Blob/Nico/gravity/BP_Goutte.BP_Goutte_C" (`KismetMathLibrary.MakeTransform` (`KismetMathLibrary.MakeVector` (+ _returnvalue_x 20.0) (+ _returnvalue_y 20.0) (+ _returnvalue_z 20.0))) "Undefined" "OverrideRootScale" null null))
    (set `self.Current Drop` _returnvalue)
    (`PrimitiveComponent.SetEnableGravity` _drops_2 false)
    (`PrimitiveComponent.SetSimulatePhysics` _drops_2 false)
    (`PrimitiveComponent.SetMaterial` _drops_2 0 "/Game/Blob/Nico/disapear/M_Dissolve.M_Dissolve")
    (bind (_direction _loc _rot) (`Timeline|Rot & Loc` :!via `PlayFromStart`)
      (:`Update`
        (`SceneComponent.K2_SetRelativeLocationAndRotation` (`self.Plane1`) (`KismetMathLibrary.MakeVector` 10.0 0.0 _loc) (`KismetMathLibrary.MakeRotator` 0.0 _rot) false false))
      (:`Finished`
        (`PrimitiveComponent.SetEnableGravity` _drops true)
        (`PrimitiveComponent.SetSimulatePhysics` _drops true)
        (`KismetSystemLibrary.Delay` 0.5)
        (bind (_direction_2 _loc_2 _rot_2) (`Timeline|Timeline_0` :!via `ReverseFromEnd`)
          (:`Update`
            (`SceneComponent.K2_SetRelativeLocationAndRotation` (`self.Plane1`) (`KismetMathLibrary.MakeVector` 10.0 0.0 _loc_2) (`KismetMathLibrary.MakeRotator` 0.0 _rot_2) false false)))))))

(fn `UserConstructionScript`)