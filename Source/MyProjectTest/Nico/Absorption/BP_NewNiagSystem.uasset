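; Test actor that attaches a Niagara system to a start capsule and passes an end capsule to it as the FinalTarget variable.
; On BeginPlay it spawns the system on CapsuleDebut and sets CapsuleFin as the target object.
; Each tick an incrementing counter drives the yaw of BlobCapsule, rotating it steadily.
; Overlap, hit and Replic handlers are empty.
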(event `self.ReceiveBeginPlay`
  (bind _returnvalue (`NiagaraFunctionLibrary.SpawnSystemAttached` "/Game/Blob/NewNiagaraSystem.NewNiagaraSystem" (`self.CapsuleDebut`) "None" (0.0 0.0 0.0) (struct) "KeepRelativeOffset"))
  (bind _output_get (set `self.Niagara` _returnvalue))
  (`NiagaraComponent.SetVariableObject` _output_get "FinalTarget" (`self.CapsuleFin`)))

(event `EnhancedInput|/Game/ThirdPerson/Input/Actions/IA_Jump`
  (params (ActionValue :type Boolean) (ElapsedSeconds :type "Float (double-precision)") (TriggeredSeconds :type "Float (double-precision)") (InputAction :type "InputAction Object Reference" :default "/Game/ThirdPerson/Input/Actions/IA_Jump.IA_Jump")))

(event `self.ReceiveTick`
  (params (DeltaSeconds :type "Float (single-precision)"))
  (bind _result (`/Engine/EditorBlueprintResources/StandardMacros.IncrementInt` (`self.cpt`))
    (:`  `
      (`SceneComponent.K2_SetRelativeRotation` (`self.BlobCapsule`) (`KismetMathLibrary.MakeRotator` 0.0 0.0 (`KismetMathLibrary.Conv_IntToDouble` (/ _result 50))) false false))))

(event `self.BlobCapsule.OnComponentHit`
  (params (HitComponent :type "PrimitiveComponent Object Reference") (OtherActor :type "Actor Object Reference") (OtherComp :type "PrimitiveComponent Object Reference") (NormalImpulse :type "Vector Structure") (Hit :type "HitResult Structure (by ref)")))

(event `EnhancedInput|/Game/ThirdPerson/Input/Actions/IA_Move`
  (params (ActionValue :type "Vector2D Structure") (ElapsedSeconds :type "Float (double-precision)") (TriggeredSeconds :type "Float (double-precision)") (InputAction :type "InputAction Object Reference" :default "/Game/ThirdPerson/Input/Actions/IA_Move.IA_Move")))

(event `EnhancedInput|/Game/ThirdPerson/Input/Actions/IA_Dash`
  (params (ActionValue :type Boolean) (ElapsedSeconds :type "Float (double-precision)") (TriggeredSeconds :type "Float (double-precision)") (InputAction :type "InputAction Object Reference" :default "/Game/ThirdPerson/Input/Actions/IA_Dash.IA_Dash")))

(event `EnhancedInput|/Game/ThirdPerson/Input/Actions/IA_CastSpellAction`
  (params (ActionValue :type "Vector2D Structure") (ElapsedSeconds :type "Float (double-precision)") (TriggeredSeconds :type "Float (double-precision)") (InputAction :type "InputAction Object Reference" :default "/Game/ThirdPerson/Input/Actions/IA_CastSpellAction.IA_CastSpellAction")))

(fn `replic`
  (params (NewParam :type Boolean)))

(fn `UserConstructionScript`)