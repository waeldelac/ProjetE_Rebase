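; BP_gravity is a potion flask actor that turns when B is pressed and drips BP_Goutte drops, with a spawned BP_Hand held above it.
; Dynamic materials on Sphere and Cylinder fake the liquid level through an "Amount" parameter driven by chained timelines.
; The chain spawns three drops at Sphere2, scaling each before enabling its gravity, then reverses the levels and loops.
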(event `self.ReceiveTick`
  (params (DeltaSeconds :type "Float (single-precision)"))
  (bind (_origin _boxextent _sphereradius) (`KismetSystemLibrary.GetComponentBounds` (`self.Flask_1`)))
  (`self.K2_SetActorRelativeLocation` (`self.MyHand`) (`KismetMathLibrary.MakeVector` (.x _origin) (.y _origin) (+ (.z _origin) _sphereradius 40.0)) false false))

(event `self.ReceiveBeginPlay`
  (bind (_origin _boxextent _sphereradius) (`KismetSystemLibrary.GetComponentBounds` (`self.Flask_1`)))
  (bind _returnvalue (`|SpawnActorFromClass` "/Game/Blob/Nico/Catchable/BP_Hand.BP_Hand_C" (`KismetMathLibrary.MakeTransform` (`KismetMathLibrary.MakeVector` (.x _origin) (.y _origin) (+ (.z _origin) _sphereradius 40.0))) "AlwaysSpawn" "OverrideRootScale" null null))
  (set `self.MyHand` _returnvalue)
  (`MaterialInstanceDynamic.SetScalarParameterValue` (`self.MatInstanceSphere`) "Amount" -0.5)
  (`MaterialInstanceDynamic.SetScalarParameterValue` (`self.MatInstanceCylinder`) "Amount" -0.5)
  (`MaterialInstanceDynamic.SetScalarParameterValue` (`self.MatInstanceCylinder`) "Amount" 0.0)
  (`MaterialInstanceDynamic.SetScalarParameterValue` (`self.MatInstanceSphere`) "Boost" 0.0)
  (`MaterialInstanceDynamic.SetScalarParameterValue` (`self.MatInstanceCylinder`) "Boost" 0.0)
  (`MaterialInstanceDynamic.SetScalarParameterValue` (`self.MatInstanceSphere`) "Fringe" 0.5)
  (`MaterialInstanceDynamic.SetScalarParameterValue` (`self.MatInstanceCylinder`) "Fringe" 0.5)
  (`MaterialInstanceDynamic.SetScalarParameterValue` (`self.MatInstanceSphere`) "Length" 2.0)
  (`MaterialInstanceDynamic.SetScalarParameterValue` (`self.MatInstanceCylinder`) "Length" 2.0)
  (`MaterialInstanceDynamic.SetScalarParameterValue` (`self.MatInstanceSphere`) "Power" 0.0001)
  (`MaterialInstanceDynamic.SetScalarParameterValue` (`self.MatInstanceCylinder`) "Power" 0.0001)
  (`MaterialInstanceDynamic.SetScalarParameterValue` (`self.MatInstanceSphere`) "TextureFade" 0.3)
  (`MaterialInstanceDynamic.SetScalarParameterValue` (`self.MatInstanceCylinder`) "TextureFade" 0.3)
  (`MaterialInstanceDynamic.SetVectorParameterValue` (`self.MatInstanceSphere`) "Base_Color" (struct :`R` 1.0 :`A` 1.0))
  (`MaterialInstanceDynamic.SetVectorParameterValue` (`self.MatInstanceCylinder`) "Base_Color" (struct :`R` 1.0 :`A` 1.0))
  (`MaterialInstanceDynamic.SetVectorParameterValue` (`self.MatInstanceSphere`) "Color" (struct :`R` 0.932292 :`G` 0.863601 :`B` 0.024499 :`A` 1.0))
  (`MaterialInstanceDynamic.SetVectorParameterValue` (`self.MatInstanceCylinder`) "Color" (struct :`R` 0.932292 :`G` 0.863601 :`B` 0.024499 :`A` 1.0))
  (`MaterialInstanceDynamic.SetVectorParameterValue` (`self.MatInstanceSphere`) "Plane" (struct :`B` 1.0 :`A` 1.0))
  (`MaterialInstanceDynamic.SetVectorParameterValue` (`self.MatInstanceCylinder`) "Plane" (struct :`B` 1.0 :`A` 1.0))
  (`MaterialInstanceDynamic.SetTextureParameterValue` (`self.MatInstanceSphere`) "None" null)
  (`MaterialInstanceDynamic.SetTextureParameterValue` (`self.MatInstanceCylinder`) "None" null)
  (`self.EnableInput` (`GameplayStatics.GetPlayerController` 0)))

(event `Key|B`
  (params (Key :type "Key Structure"))
  (bind _g3 (`self.G3`))
  (bind _g1 (`self.G1`))
  (bind (_returnvalue_x _returnvalue_y _returnvalue_z) (`KismetMathLibrary.BreakVector` (`SceneComponent.K2_GetComponentLocation` (`self.Sphere2`))))
  (bind (_returnvalue_x_2 _returnvalue_y_2 _returnvalue_z_2) (`KismetMathLibrary.BreakVector` (`SceneComponent.K2_GetComponentLocation` (`self.Sphere2`))))
  (bind (_returnvalue_x_3 _returnvalue_y_3 _returnvalue_z_3) (`KismetMathLibrary.BreakVector` (`SceneComponent.K2_GetComponentLocation` (`self.Sphere2`))))
  (:`Pressed`
    (bind (_direction _newtrack_0) (`Timeline|turn potion`)
      (:`Update`
        (`SceneComponent.K2_SetWorldRotation` (`self.DefaultSceneRoot`) (`KismetMathLibrary.MakeRotator` 0.0 (* 150 _newtrack_0)) false false)
        (`SceneComponent.K2_SetRelativeRotation` (`self.Cylinder`) (struct :`Pitch` 180.0) false false :!label _label)
        (bind (_direction_2 _newtrack_1) (`Timeline|sphere desc` :!via `PlayFromStart`)
          (:`Update`
            (`MaterialInstanceDynamic.SetScalarParameterValue` (`self.MatInstanceSphere`) "Amount" _newtrack_1)
            (if (and (not (`self.G1spawned`)) (> _newtrack_1 -0.1))
              (bind _returnvalue (`|SpawnActorFromClass` "/Game/Blob/Nico/gravity/BP_Goutte.BP_Goutte_C" (`KismetMathLibrary.MakeTransform` (`KismetMathLibrary.MakeVector` _returnvalue_x _returnvalue_y (- _returnvalue_z 2.0))) "Undefined" "OverrideRootScale" null null))
              (bind _output_get (set `self.G1` _returnvalue))
              (`PrimitiveComponent.SetEnableGravity` (`/Game/Blob/Nico/gravity/BP_Goutte.Drops` _output_get) false)
              (set `self.G1spawned` true)
              (bind (_direction_3 _newtrack_0_2) (`Timeline|scale G1` :!via `PlayFromStart`)
                (:`Update`
                  (`self.SetActorScale3D` _g1 (`KismetMathLibrary.Conv_DoubleToVector` _newtrack_0_2)))
                (:`Finished`
                  (`PrimitiveComponent.SetEnableGravity` (`/Game/Blob/Nico/gravity/BP_Goutte.Drops` _g1) true)))))
          (:`Finished`
            (set `self.G1spawned` false)
            (bind _returnvalue_2 (`|SpawnActorFromClass` "/Game/Blob/Nico/gravity/BP_Goutte.BP_Goutte_C" (`KismetMathLibrary.MakeTransform` (`KismetMathLibrary.MakeVector` _returnvalue_x_3 _returnvalue_y_3 (- _returnvalue_z_3 2.0))) "Undefined" "OverrideRootScale" null null))
            (bind _output_get_2 (set `self.G2` _returnvalue_2))
            (`PrimitiveComponent.SetEnableGravity` (`/Game/Blob/Nico/gravity/BP_Goutte.Drops` _output_get_2) false)
            (bind (_direction_4 _newtrack_1_2 _newtrack_0_3) (`Timeline|cylindre desc` :!via `PlayFromStart`)
              (:`Update`
                (`MaterialInstanceDynamic.SetScalarParameterValue` (`self.MatInstanceCylinder`) "Amount" _newtrack_1_2)
                (`self.SetActorScale3D` (`self.G2`) (`KismetMathLibrary.Conv_DoubleToVector` _newtrack_0_3))
                (if (and (not (`self.G2GravEnabled`)) (== _newtrack_0_3 1.0))
                  (`PrimitiveComponent.SetEnableGravity` (`/Game/Blob/Nico/gravity/BP_Goutte.Drops` (`self.G2`)) true)
                  (set `self.G2GravEnabled` true)))
              (:`Finished`
                (set `self.G2GravEnabled` false)
                (bind _returnvalue_3 (`|SpawnActorFromClass` "/Game/Blob/Nico/gravity/BP_Goutte.BP_Goutte_C" (`KismetMathLibrary.MakeTransform` (`KismetMathLibrary.MakeVector` _returnvalue_x_2 _returnvalue_y_2 (- _returnvalue_z_2 2.0))) "Undefined" "OverrideRootScale" null null))
                (bind _output_get_3 (set `self.G3` _returnvalue_3))
                (`PrimitiveComponent.SetEnableGravity` (`/Game/Blob/Nico/gravity/BP_Goutte.Drops` _output_get_3) false)
                (bind (_direction_5 _newtrack_0_4) (`Timeline|scale G3` :!via `PlayFromStart`)
                  (:`Update`
                    (`self.SetActorScale3D` _g3 (`KismetMathLibrary.Conv_DoubleToVector` _newtrack_0_4)))
                  (:`Finished`
                    (`PrimitiveComponent.SetEnableGravity` (`/Game/Blob/Nico/gravity/BP_Goutte.Drops` _g3) true)
                    (`SceneComponent.K2_SetRelativeRotation` (`self.Cylinder`) (struct :`Pitch` 180.0) false false)
                    (bind (_direction_6 _newtrack_1_3) (`Timeline|cylindre mont` :!via `ReverseFromEnd`)
                      (:`Update`
                        (`MaterialInstanceDynamic.SetScalarParameterValue` (`self.MatInstanceCylinder`) "Amount" _newtrack_1_3))
                      (:`Finished`
                        (bind (_direction_7 _newtrack_1_4) (`Timeline|sphere mont` :!via `ReverseFromEnd`)
                          (:`Update`
                            (`MaterialInstanceDynamic.SetScalarParameterValue` (`self.MatInstanceSphere`) "Amount" _newtrack_1_4))
                          (:`Finished`
                            (goto _label)))))))))))))))

(event `Key|V`
  (params (Key :type "Key Structure")))

(fn `UserConstructionScript`
  (bind _returnvalue (`PrimitiveComponent.CreateDynamicMaterialInstance` (`self.Sphere`) 0 null "None"))
  (set `self.MatInstanceSphere` _returnvalue)
  (bind _returnvalue_2 (`PrimitiveComponent.CreateDynamicMaterialInstance` (`self.Cylinder`) 0 null "None"))
  (set `self.MatInstanceCylinder` _returnvalue_2))