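; Generated dynamic mesh actor that prototypes ice and water elements, with only the water part currently running.
; On rebuild, AddElements copies a static water mesh into DynamicWater, applies its material and issues a scaled transform at the target coordinates.
; Ice creation and cylinder boolean subtraction for carving the ice are disconnected, leaving ComputeShape empty.
; The ice overlap event only reads the other dynamic mesh actor's transform.
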(event `self.OnRebuildGeneratedMesh`
  (params (TargetMesh :type "DynamicMesh Object Reference"))
  (`self.Add elements` (`self.Target X`) (`self.Target Y`) (`self.Target Z`)))

(event `self.ReceiveTick`
  (params (DeltaSeconds :type "Float (single-precision)")))

(event `self.Dynamic_Ice.OnComponentBeginOverlap`
  (params (OverlappedComponent :type "PrimitiveComponent Object Reference") (OtherActor :type "Actor Object Reference") (OtherComp :type "PrimitiveComponent Object Reference") (OtherBodyIndex :type Integer) (bFromSweep :type Boolean) (SweepResult :type "HitResult Structure (by ref)"))
  (bind _asdynamic_mesh_actor (cast `DynamicMeshActor` OtherActor))
  (bind _outtransform (message `TypedElementWorldInterface.GetWorldTransform` _asdynamic_mesh_actor (`self.In Element Handle`))))

(fn `Add elements`
  (params (X :type "Float (double-precision)") (Y :type "Float (double-precision)") (Z :type "Float (double-precision)"))
  ;[1 1 1] add water
  (bind _returnvalue (`BaseDynamicMeshComponent.GetDynamicMesh` (`self.Dynamic_Water`)))
  (`GeometryScriptLibrary_StaticMeshFunctions.CopyMeshFromStaticMesh` (`self.static_water`) _returnvalue (struct) (struct) null
    (:`Success`
      (`PrimitiveComponent.SetMaterial` (`self.Dynamic_Water`) 0 "/DatasmithContent/Materials/Water/M_Water.M_Water")
      (bind _returnvalue_2 (`BaseDynamicMeshComponent.GetDynamicMesh` (`self.DynamicMeshComponent`)))
      (message `TypedElementWorldInterface.SetRelativeTransform` _returnvalue_2 (`self.In Element Handle`) (`KismetMathLibrary.MakeTransform` (`KismetMathLibrary.MakeVector` X Y Z) (struct) (2.0 2.0 0.5))))))

(fn `Compute shape`
  (params (tool_cylinderX :type "Float (double-precision)") (tool_cylinderY :type "Float (double-precision)") (tool_cylinderZ :type "Float (double-precision)") (target_cylinderX :type "Float (double-precision)") (target_cylinderY :type "Float (double-precision)") (target_cylinderZ :type "Float (double-precision)")))

(fn `UserConstructionScript`)