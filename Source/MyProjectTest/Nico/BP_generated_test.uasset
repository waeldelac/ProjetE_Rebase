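; Test generated-mesh actor that builds a flat ice box and keeps punching holes in it.
; Rebuild cuts three fixed holes, then Tick adds one at a random offset every 100 frames, refreshing collision.
; CreateHole subtracts a cylinder with a Geometry Script boolean and spawns an attached BP_generated_ice there.
; ComputeHoles, meant to reshape ice pieces against each other and track them, is disconnected, leaving the cleanup array unfilled.
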(event `Key|LeftMouseButton`
  (params (Key :type "Key Structure")))

(event `Key|B`
  (params (Key :type "Key Structure")))

(event `self.ReceiveBeginPlay`
  (for _array_element (`self.Array BP_generated_Ice`)
    (`self.K2_DestroyActor` _array_element))
  (`KismetArrayLibrary.Array_Clear` (`self.Array BP_generated_Ice`)))

(event `self.ReceiveTick`
  (params (DeltaSeconds :type "Float (single-precision)"))
  (bind _cpt (`self.cpt`))
  (`/Engine/EditorBlueprintResources/StandardMacros.IncrementInt` _cpt
    (:`  `
      (if (== (mod _cpt 100) 1)
        (`self.part hole creation`)))))

(event `self.OnRebuildGeneratedMesh`
  (params (TargetMesh :type "DynamicMesh Object Reference"))
  (set `self.Target Mesh` TargetMesh)
  (for _array_element (`self.Array BP_generated_Ice`)
    (`self.K2_DestroyActor` _array_element))
  (`KismetArrayLibrary.Array_Clear` (`self.Array BP_generated_Ice`))
  (`GeometryScriptLibrary_MeshPrimitiveFunctions.AppendBox` (`self.Target Mesh`) (make `GeometryScriptPrimitiveOptions` "PerFace") (`KismetMathLibrary.MakeTransform` (`KismetMathLibrary.MakeVector` (`self.Transform Location X`) (`self.Transform Location Y`) (`self.Transform Location Z`)) (struct) (10.0 10.0 0.1)) 100.0 100.0 100.0 0 0 0 "Base" null)
  (`PrimitiveComponent.SetMaterial` (`self.DynamicMeshComponent`) 0 "/Game/InfinityBladeIceLands/Environments/Ice/Env_Ice_Terrain/Materials/M_Ice_VertPaint.M_Ice_VertPaint")
  (bind _returnvalue (`BaseDynamicMeshComponent.GetDynamicMesh` (`self.DynamicMeshComponent`)))
  (`self.create hole` _returnvalue 100.0 100.0 0.0)
  (`self.create hole` _returnvalue 100.0 110.0 0.0)
  (`self.create hole` _returnvalue 150.0 120.0 0.0)
  (`DynamicMeshComponent.UpdateCollision` (`self.DynamicMeshComponent`) true))

(event `self.DynamicMeshComponent.OnComponentBeginOverlap`
  (params (OverlappedComponent :type "PrimitiveComponent Object Reference") (OtherActor :type "Actor Object Reference") (OtherComp :type "PrimitiveComponent Object Reference") (OtherBodyIndex :type Integer) (bFromSweep :type Boolean) (SweepResult :type "HitResult Structure (by ref)"))
  (`KismetSystemLibrary.PrintString` "Youpi" :!label _label))

(event `self.DynamicMeshComponent.OnComponentHit`
  (params (HitComponent :type "PrimitiveComponent Object Reference") (OtherActor :type "Actor Object Reference") (OtherComp :type "PrimitiveComponent Object Reference") (NormalImpulse :type "Vector Structure") (Hit :type "HitResult Structure (by ref)"))
  (goto _label))

(fn `Compute Holes`
  (params (`Last BP_generated_Ice` :type "/Game/Blob/Nico/BP_generated_ice Object Reference"))
  (locals (`local Current BP_Generated_Ice` :type "/Game/Blob/Nico/BP_generated_ice Object Reference") (`last BP_Generated_Ice element` :type "/Game/Blob/Nico/BP_generated_ice Object Reference"))
  (bind _returnvalue_location (`self.get current element position`))
  (bind _returnvalue_location_2 (`self.get last array element position`))
  (bind _returnvalue_location_3 (`self.get current element position`))
  (bind _returnvalue_location_4 (`self.get last array element position`))
  (set `local.last BP_Generated_Ice element` `Last BP_generated_Ice`)
  (if (> (`KismetArrayLibrary.Array_Length` (`self.Array BP_generated_Ice`)) 0)
    (for (_array_element _array_index) (`self.Array BP_generated_Ice`)
      (`KismetSystemLibrary.PrintString` (`KismetStringLibrary.Conv_IntToString` _array_index))
      (set `local.local Current BP_Generated_Ice` _array_element)
      (`/Game/Blob/Nico/BP_generated_ice.Compute shape` (`local.last BP_Generated_Ice element`) (.x _returnvalue_location) (.y _returnvalue_location) (.z _returnvalue_location) (.x _returnvalue_location_2) (.y _returnvalue_location_2) (.z _returnvalue_location_2))
      (`/Game/Blob/Nico/BP_generated_ice.Compute shape` (`local.local Current BP_Generated_Ice`) (.x _returnvalue_location_4) (.y _returnvalue_location_4) (.z _returnvalue_location_4) (.x _returnvalue_location_3) (.y _returnvalue_location_3) (.z _returnvalue_location_3)))
    (`KismetArrayLibrary.Array_Add` (`self.Array BP_generated_Ice`) (`local.last BP_Generated_Ice element`))
    (else
      (`KismetArrayLibrary.Array_Add` (`self.Array BP_generated_Ice`) (`local.last BP_Generated_Ice element`)))))

(fn `create hole`
  (params (TargetMesh :type "DynamicMesh Object Reference") (X :type "Float (double-precision)") (Y :type "Float (double-precision)") (Z :type "Float (double-precision)"))
  (bind _returnvalue (`KismetMathLibrary.MakeVector` X Y Z))
  (bind _returnvalue_2 (`self.AllocateComputeMesh`))
  (bind _returnvalue_3 (`GeometryScriptLibrary_MeshPrimitiveFunctions.AppendCylinder` _returnvalue_2 (struct) (`KismetMathLibrary.MakeTransform` (`KismetMathLibrary.MakeVector` X Y Z) (struct) (1.0 1.0 100.0)) 50.0 2000000.0 100 0 true "Base" null))
  (bind _returnvalue_4 (`GeometryScriptLibrary_MeshBooleanFunctions.ApplyMeshBoolean` TargetMesh (struct) _returnvalue_3 (struct) "Subtract" (struct) null))
  (`self.ReleaseComputeMesh` _returnvalue_4)
  (bind _returnvalue_5 (`|SpawnActorFromClass` "/Game/Blob/Nico/BP_generated_ice.BP_generated_ice_C" (`KismetMathLibrary.MakeTransform` _returnvalue) "Undefined" "MultiplyWithRoot" null null))
  (`/Game/Blob/Nico/BP_generated_ice.Add elements` _returnvalue_5 X Y Z)
  (`self.K2_AttachToComponent` _returnvalue_5 (`self.DynamicMeshComponent`) "None" "KeepRelative" "KeepRelative" "KeepRelative" true)
  (bind _returnvalue_6 (`BaseDynamicMeshComponent.GetDynamicMesh` (`DynamicMeshActor.DynamicMeshComponent` _returnvalue_5)))
  (message `TypedElementWorldInterface.SetRelativeTransform` _returnvalue_6 (`self.In Element Handle`) (`KismetMathLibrary.MakeTransform` _returnvalue)))

(fn `part hole creation`
  (bind _returnvalue (`BaseDynamicMeshComponent.GetDynamicMesh` (`self.DynamicMeshComponent`)))
  (`self.create hole` _returnvalue (+ (`self.Transform Location X`) (`KismetMathLibrary.RandomIntegerInRange` -400 400)) (+ (`self.Transform Location Y`) (`KismetMathLibrary.RandomIntegerInRange` -400 400)) (`self.Transform Location Z`))
  (`DynamicMeshComponent.UpdateCollision` (`self.DynamicMeshComponent`) true))

(fn `UserConstructionScript`)